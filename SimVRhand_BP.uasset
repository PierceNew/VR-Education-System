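; SimVRhand_BP is a VR hand actor that grabs and drops objects, with the hand mesh mirrored on Y for the left hand.
; Grab takes the first actor overlapping its Sphere, casts it to GrabBable and passes it the hand mesh; Drop notifies that stored target.
; GetHandState reports idle, grabbable in range or grab pressed as a float.
; BeginPlay caches the mesh's HandAim_BP anim instance.
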(event `self.ReceiveBeginPlay`
  (bind _ashand_aim_bp (cast `/Game/Player/moni/PCcontrol/HandAim_BP` (`SkeletalMeshComponent.GetAnimInstance` (`self.HandMesh`))))
  (set `self.HandAim` _ashand_aim_bp))

(event `self.Sphere.OnComponentBeginOverlap`
  (params (OverlappedComponent :type "PrimitiveComponent Object Reference") (OtherActor :type "Actor Object Reference") (OtherComp :type "PrimitiveComponent Object Reference") (OtherBodyIndex :type Integer) (bFromSweep :type Boolean) (SweepResult :type "HitResult Structure (by ref)")))

(event `self.Sphere.OnComponentEndOverlap`
  (params (OverlappedComponent :type "PrimitiveComponent Object Reference") (OtherActor :type "Actor Object Reference") (OtherComp :type "PrimitiveComponent Object Reference") (OtherBodyIndex :type Integer)))

(fn `Drop`
  (bind _grabtarget (`self.GrabTarget`))
  (set `self.isGrabPressed` false)
  (`/Engine/EditorBlueprintResources/StandardMacros.IsValid` (`KismetSystemLibrary.Conv_InterfaceToObject` _grabtarget)
    (:`Is Valid`
      (`/Game/Player/moni/shiqulei/GrabBable.OnDrop` _grabtarget))))

(fn `FindGrabTarget`
  (returns (GrabTarget :type "/Game/Player/moni/shiqulei/GrabBable Interface"))
  (bind _sphere (`self.Sphere`))
  (`/Engine/EditorBlueprintResources/StandardMacros.IsValid` _sphere
    (:`Is Valid`
      (bind _asgrab_bable (cast `/Game/Player/moni/shiqulei/GrabBable` (`|GetArrayItem` (`PrimitiveComponent.GetOverlappingActors` _sphere null))))
      (return _asgrab_bable))))

(fn `GetHandState`
  (returns (State :type "Float (double-precision)"))
  (if (`self.isGrabPressed`)
    (return 2.0)
    (else
      (`/Engine/EditorBlueprintResources/StandardMacros.IsValid` (`KismetSystemLibrary.Conv_InterfaceToObject` (`self.FindGrabTarget`))
        (:`Is Valid`
          (return 1.0))
        (:`Is Not Valid`
          (return 0.0))))))

(fn `Grab`
  (set `self.isGrabPressed` true)
  (bind _output_get (set `self.GrabTarget` (`self.FindGrabTarget`)))
  (`/Engine/EditorBlueprintResources/StandardMacros.IsValid` (`KismetSystemLibrary.Conv_InterfaceToObject` _output_get)
    (:`Is Valid`
      (`/Game/Player/moni/shiqulei/GrabBable.OnGrab` _output_get (`self.HandMesh`)))))

(fn `UserConstructionScript`
  (if (`self.isLeft`)
    (`SceneComponent.SetWorldScale3D` (`self.HandMesh`) (1.0 -1.0 1.0))))
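; A grabbable disinfectant sprayer for the SimVR_BP player that damages bingdu_BP (virus) actors.
; Grabbing attaches it to the hand with an arrow-based offset and shows weapon and usage UI; dropping restores physics and removes the UI.
; Fire sphere-traces briefly from its Muzzle, subtracting the virus's own Damge from its HP, but spawns the particle effect at the player's AK muzzle socket.
; Custom depth on its meshes toggles an outline.
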(event `self.ReceiveBeginPlay`
  (`PrimitiveComponent.SetRenderCustomDepth` (`self.Object___`) false)
  (`PrimitiveComponent.SetRenderCustomDepth` (`self.Object___1`) false)
  (`PrimitiveComponent.SetRenderCustomDepth` (`self.Object___2`) false)
  (`PrimitiveComponent.SetRenderCustomDepth` (`self.Object___3`) false)
  (`PrimitiveComponent.SetRenderCustomDepth` (`self.StaticMesh1`) false)
  (bind _assim_vr_bp (cast `/Game/Player/moni/PCcontrol/SimVR_BP` (`GameplayStatics.GetPlayerCharacter` 0)))
  (set `self.player` _assim_vr_bp))

(event `/Game/Player/moni/shiqulei/GrabBable.OnGrab`
  (params (Hand :type "SceneComponent Object Reference"))
  (bind _staticmesh (`self.StaticMesh`))
  (bind _arrow (`self.Arrow`))
  (`PrimitiveComponent.SetSimulatePhysics` (`self.StaticMesh`) false)
  (`self.K2_AttachToComponent` Hand "None" "KeepWorld" "KeepWorld" "KeepWorld")
  (set `self.IsCatch?` true)
  (`SceneComponent.K2_SetRelativeLocation` _staticmesh (* (`SceneComponent.RelativeLocation` _arrow) -1.0) false false)
  (`SceneComponent.K2_SetRelativeRotation` _staticmesh (`KismetMathLibrary.NegateRotator` (`SceneComponent.RelativeRotation` _arrow)) false false)
  (`/Game/HUD/CLass3fangjian/weapen_HUD.消毒器` (`/Game/Player/moni/PCcontrol/SimVR_BP.weaponUI` (`self.player`)))
  (bind _returnvalue (`|CreateWidget` "/Game/HUD/CLass3fangjian/Use喷雾器.Use喷雾器_C"))
  (`UserWidget.AddToViewport` _returnvalue 0)
  (`/Game/HUD/CLass3fangjian/Use喷雾器.shank` _returnvalue)
  (`KismetSystemLibrary.Delay` 5.0)
  (`/Game/HUD/CLass3fangjian/Use喷雾器.Destory` _returnvalue))

(event `/Game/Player/moni/shiqulei/GrabBable.OnDrop`
  (bind _staticmesh (`self.StaticMesh`))
  (`PrimitiveComponent.SetSimulatePhysics` _staticmesh true)
  (`SceneComponent.K2_DetachFromComponent` _staticmesh "KeepWorld" "KeepWorld" "KeepWorld" true)
  (set `self.IsCatch?` false)
  (set `self.isfire` false)
  (`/Game/HUD/CLass3fangjian/weapen_HUD.destory消毒器` (`/Game/Player/moni/PCcontrol/SimVR_BP.weaponUI` (`self.player`)))
  (`Widget.RemoveFromParent` (stale `/Game/Player/moni/shiqulei/GrabBable.OnGrab` _returnvalue)))

(event `Fire`
  (bind _muzzle (`self.Muzzle`))
  (bind _returnvalue (`SceneComponent.K2_GetComponentLocation` _muzzle))
  (set `self.isfire` true)
  (bind _assim_vr_bp (cast `/Game/Player/moni/PCcontrol/SimVR_BP` (`GameplayStatics.GetPlayerCharacter` 0)))
  (bind _muzzle_2 (`/penwuqi_BP.Muzzle` (`/Game/Player/moni/PCcontrol/SimVR_BP.AK` _assim_vr_bp)))
  ;[1 1 1] 发射特效
  (bind _returnvalue_2 (`GameplayStatics.SpawnEmitterAtLocation` "/Game/MobileStarterContent/Particles/P_Explosion.P_Explosion" (`SceneComponent.GetSocketLocation` _muzzle_2 "Muzzle") (`SceneComponent.GetSocketRotation` _muzzle_2 "Muzzle")))
  (`SceneComponent.SetWorldScale3D` _returnvalue_2 (0.3 0.3 0.5))
  ;[1 1 1] 消毒扣血
  (bind _outhit (`KismetSystemLibrary.SphereTraceSingle` _returnvalue (+ _returnvalue (* (`SceneComponent.GetForwardVector` _muzzle) 100.0)) 10.0 "TraceTypeQuery1"))
  (bind _asbingdu_bp (cast `/Game/Mission_BP/bingdu/bingdu_BP` (`.HitActor` (`GameplayStatics.BreakHitResult` _outhit))))
  (set `/Game/Mission_BP/bingdu/bingdu_BP.currentHP` (- (`/Game/Mission_BP/bingdu/bingdu_BP.currentHP` _asbingdu_bp) (`/Game/Mission_BP/bingdu/bingdu_BP.Damge` _asbingdu_bp)) _asbingdu_bp))

(event `OpenOutline`
  (`PrimitiveComponent.SetRenderCustomDepth` (`self.Object___`) true)
  (`PrimitiveComponent.SetRenderCustomDepth` (`self.Object___3`) true)
  (`PrimitiveComponent.SetRenderCustomDepth` (`self.Object___2`) true)
  (`PrimitiveComponent.SetRenderCustomDepth` (`self.Object___1`) true)
  (`PrimitiveComponent.SetRenderCustomDepth` (`self.StaticMesh1`) true))

(event `CloseOutline`
  (bind _object___ (`self.Object___`))
  (bind _object___1 (`self.Object___1`))
  (bind _object___2 (`self.Object___2`))
  (bind _object___3 (`self.Object___3`))
  (bind _staticmesh1 (`self.StaticMesh1`))
  (`|ExecutionSequence`
    (:`then_0`
      (if (`PrimitiveComponent.bRenderCustomDepth` _object___)
        (`PrimitiveComponent.SetRenderCustomDepth` _object___ false)))
    (:`then_1`
      (if (`PrimitiveComponent.bRenderCustomDepth` _object___3)
        (`PrimitiveComponent.SetRenderCustomDepth` _object___3 false)))
    (:`then_2`
      (if (`PrimitiveComponent.bRenderCustomDepth` _object___2)
        (`PrimitiveComponent.SetRenderCustomDepth` _object___2 false)))
    (:`then_3`
      (if (`PrimitiveComponent.bRenderCustomDepth` _object___1)
        (`PrimitiveComponent.SetRenderCustomDepth` _object___1 false)))
    (:`then_4`
      (if (`PrimitiveComponent.bRenderCustomDepth` _staticmesh1)
        (`PrimitiveComponent.SetRenderCustomDepth` _staticmesh1 false)))))

(fn `UserConstructionScript`)
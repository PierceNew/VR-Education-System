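; NPC2_BP is an NPC that wanders between random Trigger actors and reacts in surprise when the SimVR_BP actor overlaps its box.
; BeginPlay caches the triggers and loops AIMoveTo to random ones until the 撞到了 (bumped) flag is set.
; On overlap it halts by moving to itself, turns toward the intruder, shows text and plays a surprise montage via NPC2_Aim.
; After a delay it resets and resumes wandering.
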(event `self.ReceiveBeginPlay`
  (`|ExecutionSequence`
    (:`then_0`
      (bind _outactors (`GameplayStatics.GetAllActorsOfClass` "/Game/Player/moni/NPC/trigger.trigger_C"))
      (set `self.目标点` _outactors))
    (:`then_1`
      (`|AIMoveTo` self (0.0 0.0 0.0) (`self.GetRandomWaypoint`) :!label _label
        (:`OnSuccess`
          _)
        (:`OnFail`
          _))
      (if (not (`self.撞到了`))
        (goto _label)))
    (:`then_2`
      (`SceneComponent.SetVisibility` (`self.TextRender`) false false))
    (:`then_3`
      (bind _asnpc2_aim (cast `/Game/Player/moni/NPC/NPC2_Aim` (`SkeletalMeshComponent.GetAnimInstance` (`self.Mesh`))))
      (set `self.NPC2_Aim` _asnpc2_aim))))

(event `self.ReceiveTick`
  (params (DeltaSeconds :type "Float (single-precision)")))

(event `self.Box.OnComponentBeginOverlap`
  (params (OverlappedComponent :type "PrimitiveComponent Object Reference") (OtherActor :type "Actor Object Reference") (OtherComp :type "PrimitiveComponent Object Reference") (OtherBodyIndex :type Integer) (bFromSweep :type Boolean) (SweepResult :type "HitResult Structure (by ref)"))
  (bind _npc2_aim (`self.NPC2_Aim`))
  (bind _assim_vr_bp (cast `/Game/Player/moni/PCcontrol/SimVR_BP` OtherActor))
  (set `self.撞到了` true)
  (`|ExecutionSequence`
    (:`then_0`
      (`SceneComponent.SetVisibility` (`self.TextRender`) true false))
    (:`then_1`
      (`|AIMoveTo` self (0.0 0.0 0.0) self))
    (:`then_2`
      (`self.K2_SetActorRotation` (`KismetMathLibrary.RLerp` (`self.K2_GetActorRotation`) (`KismetMathLibrary.FindLookAtRotation` (`self.K2_GetActorLocation`) (`self.K2_GetActorLocation` _assim_vr_bp)) 0.8)))
    (:`then_3`
      (set `/Game/Player/moni/NPC/NPC2_Aim.suprised?` true _npc2_aim)
      (`AnimInstance.Montage_Play` (`SkeletalMeshComponent.GetAnimInstance` (`self.Mesh`)) "/Game/Player/moni/NPC/1/AIM/Surprised_NPC1_Montage.Surprised_NPC1_Montage" 1.0 "MontageLength" 0.0 false)
      (`KismetSystemLibrary.Delay` 4.0)
      (set `/Game/Player/moni/NPC/NPC2_Aim.suprised?` false _npc2_aim)
      ;[1 1 1] 等待后恢复
      (set `self.撞到了` false)
      (`SceneComponent.SetVisibility` (`self.TextRender`) false false)
      (`|AIMoveTo` self (0.0 0.0 0.0) (`self.GetRandomWaypoint`) :!label _label_2
        (:`OnSuccess`
          _)
        (:`OnFail`
          _))
      (if (not (`self.撞到了`))
        (goto _label_2)))))

(fn `GetRandomWaypoint`
  (returns (Output :type "/Game/Player/moni/NPC/trigger Object Reference"))
  (bind `_目标点` (`self.目标点`))
  (return (`|GetArrayItem` `_目标点` (`KismetMathLibrary.RandomIntegerInRange` 0 (- (`KismetArrayLibrary.Array_Length` `_目标点`) 1)))))

(fn `UserConstructionScript`)
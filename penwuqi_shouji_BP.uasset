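; Grabbable prop Blueprint, apparently a sprayer going by the asset name, that can be picked up by hand and highlighted.
; OnGrab turns off physics and collision, attaches to the passed hand keeping world transform, and sets IsCatch.
; OnDrop detaches, restores physics and collision, and clears the flag.
; OpenOutline and CloseOutline toggle the mesh's custom depth rendering for an outline, which starts off at BeginPlay.
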(event `self.ReceiveBeginPlay`
  (`PrimitiveComponent.SetRenderCustomDepth` (`self.mesh`) false))

(event `/Game/Player/moni/shiqulei/GrabBable.OnGrab`
  (params (Hand :type "SceneComponent Object Reference"))
  (bind _mesh (`self.mesh`))
  (`PrimitiveComponent.SetSimulatePhysics` _mesh false)
  (`self.K2_AttachToComponent` Hand "None" "KeepWorld" "KeepWorld" "KeepWorld")
  (set `self.IsCatch?` true)
  (`PrimitiveComponent.SetCollisionEnabled` _mesh "NoCollision"))

(event `/Game/Player/moni/shiqulei/GrabBable.OnDrop`
  (bind _mesh (`self.mesh`))
  (`PrimitiveComponent.SetSimulatePhysics` _mesh true)
  (`SceneComponent.K2_DetachFromComponent` _mesh "KeepWorld" "KeepWorld" "KeepWorld" true)
  (set `self.IsCatch?` false)
  (`PrimitiveComponent.SetCollisionEnabled` _mesh "QueryAndPhysics"))

(event `OpenOutline`
  (`PrimitiveComponent.SetRenderCustomDepth` (`self.mesh`) true))

(event `CloseOutline`
  (bind _mesh (`self.mesh`))
  (if (`PrimitiveComponent.bRenderCustomDepth` _mesh)
    (`PrimitiveComponent.SetRenderCustomDepth` _mesh false)))

(fn `UserConstructionScript`)
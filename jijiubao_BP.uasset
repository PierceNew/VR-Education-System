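; First-aid kit ("jijiubao") actor that can be grabbed and dropped by a hand and highlighted with an outline.
; Grabbing turns off mesh physics and attaches to the hand at its current world transform, while dropping detaches and re-enables physics, with IsCatch tracking the held state.
; OpenOutline and CloseOutline toggle the mesh's Render Custom Depth for highlighting, which starts off at BeginPlay.
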(event `self.ReceiveBeginPlay`
  (`PrimitiveComponent.SetRenderCustomDepth` (`self.StaticMesh`) false))

(event `/Game/Player/moni/shiqulei/GrabBable.OnGrab`
  (params (Hand :type "SceneComponent Object Reference"))
  (`PrimitiveComponent.SetSimulatePhysics` (`self.StaticMesh`) false)
  (`self.K2_AttachToComponent` Hand "None" "KeepWorld" "KeepWorld" "KeepWorld")
  (set `self.IsCatch?` true))

(event `/Game/Player/moni/shiqulei/GrabBable.OnDrop`
  (bind _staticmesh (`self.StaticMesh`))
  (`PrimitiveComponent.SetSimulatePhysics` _staticmesh true)
  (`SceneComponent.K2_DetachFromComponent` _staticmesh "KeepWorld" "KeepWorld" "KeepWorld" true)
  (set `self.IsCatch?` false))

(event `OpenOutline`
  (`PrimitiveComponent.SetRenderCustomDepth` (`self.StaticMesh`) true))

(event `CloseOutline`
  (bind _staticmesh (`self.StaticMesh`))
  (if (`PrimitiveComponent.bRenderCustomDepth` _staticmesh)
    (`PrimitiveComponent.SetRenderCustomDepth` _staticmesh false)))

(fn `UserConstructionScript`)
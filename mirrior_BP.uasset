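; Mirror trigger actor that manages a Check_HUD widget as the SimVR_BP actor enters and leaves its box.
; On begin overlap it shows the widget if that actor's 碰到镜子了 ("touched mirror") flag is already set, then sets the flag, so a first touch with a cleared flag only arms it.
; On end overlap it destroys the widget and clears the flag only if the flag is already false.
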(event `self.Box.OnComponentBeginOverlap`
  (params (OverlappedComponent :type "PrimitiveComponent Object Reference") (OtherActor :type "Actor Object Reference") (OtherComp :type "PrimitiveComponent Object Reference") (OtherBodyIndex :type Integer) (bFromSweep :type Boolean) (SweepResult :type "HitResult Structure (by ref)"))
  (bind _assim_vr_bp (cast `/Game/Player/moni/PCcontrol/SimVR_BP` OtherActor))
  (`|ExecutionSequence`
    (:`then_0`
      (if (`/Game/Player/moni/PCcontrol/SimVR_BP.碰到镜子了` _assim_vr_bp)
        (bind _returnvalue (`|CreateWidget` "/Game/HUD/Class2_wuzishi/check_HUD.check_HUD_C"))
        (`UserWidget.AddToViewport` _returnvalue 0)))
    (:`then_1`
      (set `/Game/Player/moni/PCcontrol/SimVR_BP.碰到镜子了` true _assim_vr_bp))))

(event `self.Box.OnComponentEndOverlap`
  (params (OverlappedComponent :type "PrimitiveComponent Object Reference") (OtherActor :type "Actor Object Reference") (OtherComp :type "PrimitiveComponent Object Reference") (OtherBodyIndex :type Integer))
  (bind _assim_vr_bp (cast `/Game/Player/moni/PCcontrol/SimVR_BP` OtherActor))
  (if (not (`/Game/Player/moni/PCcontrol/SimVR_BP.碰到镜子了` _assim_vr_bp))
    (`/Game/HUD/Class2_wuzishi/check_HUD.destory` (stale `self.Box.OnComponentBeginOverlap` _returnvalue))
    (set `/Game/Player/moni/PCcontrol/SimVR_BP.碰到镜子了` false _assim_vr_bp)))

(fn `UserConstructionScript`)
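; VR grabbable temperature gun (测温枪) that takes a temperature reading from an NPC.
; Grabbing attaches it to the hand using the inverted Arrow offset and shows its widget and player weapon UI; dropping restores physics and clears both.
; 测温 briefly blanks that widget and sphere-traces from the Arrow for NPC4_BP; hits flash a second widget and, once only, notify the level via a "ce 完成测温" console command.
; Custom depth provides the highlight outline.
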(event `self.ReceiveBeginPlay`
  (set `self.IsCatch?` false)
  (`PrimitiveComponent.SetRenderCustomDepth` (`self.StaticMesh`) false)
  (`SceneComponent.SetVisibility` (`self.Widget`) false false)
  (bind _assim_vr_bp (cast `/Game/Player/moni/PCcontrol/SimVR_BP` (`GameplayStatics.GetPlayerCharacter` 0)))
  (set `self.player` _assim_vr_bp))

(event `/Game/Player/moni/shiqulei/GrabBable.OnGrab`
  (params (Hand :type "SceneComponent Object Reference"))
  (bind _staticmesh (`self.StaticMesh`))
  (bind _arrow (`self.Arrow`))
  (`PrimitiveComponent.SetSimulatePhysics` (`self.StaticMesh`) false)
  (`self.K2_AttachToComponent` Hand "None" "KeepWorld" "KeepWorld" "KeepWorld")
  (set `self.IsCatch?` true)
  (`SceneComponent.K2_SetRelativeLocation` _staticmesh (* (`SceneComponent.RelativeLocation` _arrow) -1.0) false false)
  (`SceneComponent.K2_SetRelativeRotation` _staticmesh (`KismetMathLibrary.NegateRotator` (`SceneComponent.RelativeRotation` _arrow)) false false)
  (bind _returnvalue (`|CreateWidget` "/Game/HUD/CLass3fangjian/E测温.E测温_C"))
  (`WidgetComponent.SetWidget` (`self.Widget1`) _returnvalue)
  (`/Game/HUD/CLass3fangjian/weapen_HUD.测温枪` (`/Game/Player/moni/PCcontrol/SimVR_BP.weaponUI` (`self.player`))))

(event `/Game/Player/moni/shiqulei/GrabBable.OnDrop`
  (bind _staticmesh (`self.StaticMesh`))
  (`PrimitiveComponent.SetSimulatePhysics` _staticmesh true)
  (`SceneComponent.K2_DetachFromComponent` _staticmesh "KeepWorld" "KeepWorld" "KeepWorld" true)
  (set `self.IsCatch?` false)
  (set `self.isfire` false)
  (`WidgetComponent.SetWidget` (`self.Widget1`) null)
  (`/Game/HUD/CLass3fangjian/weapen_HUD.destory测温枪` (`/Game/Player/moni/PCcontrol/SimVR_BP.weaponUI` (`self.player`))))

(event `OpenOutline`
  (`PrimitiveComponent.SetRenderCustomDepth` (`self.StaticMesh`) true))

(event `CloseOutline`
  (bind _staticmesh (`self.StaticMesh`))
  (if (`PrimitiveComponent.bRenderCustomDepth` _staticmesh)
    (`PrimitiveComponent.SetRenderCustomDepth` _staticmesh false)))

(event `测温`
  (bind _widget (`self.Widget`))
  (bind _arrow (`self.Arrow`))
  (bind _returnvalue (`SceneComponent.K2_GetComponentLocation` _arrow))
  (`|ExecutionSequence`
    (:`then_0`
      (`WidgetComponent.SetWidget` (`self.Widget1`) null)
      (`KismetSystemLibrary.Delay` 4.0)
      (`WidgetComponent.SetWidget` (`self.Widget1`) (stale `/Game/Player/moni/shiqulei/GrabBable.OnGrab` _returnvalue)))
    (:`then_1`
      (bind _outhit (`KismetSystemLibrary.SphereTraceSingle` _returnvalue (+ _returnvalue (* (`SceneComponent.GetForwardVector` _arrow) 100.0)) 10.0 "TraceTypeQuery1"))
      (cast `/Game/Player/moni/NPC/4/NPC4_BP` (`.HitActor` (`GameplayStatics.BreakHitResult` _outhit)))
      (`|ExecutionSequence`
        (:`then_0`
          (`/Engine/EditorBlueprintResources/StandardMacros.DoOnce` false :!label _label
            (:`Completed`
              (`SceneComponent.SetVisibility` _widget true false)
              (`KismetSystemLibrary.Delay` 3.0)
              (`SceneComponent.SetVisibility` _widget false false)
              (goto _label :!via `Reset`))))
        (:`then_1`
          (`/Engine/EditorBlueprintResources/StandardMacros.DoOnce` false
            (:`Completed`
              (`KismetSystemLibrary.ExecuteConsoleCommand` "ce 完成测温" null))))))))

(fn `UserConstructionScript`)
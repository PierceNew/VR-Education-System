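; humujing_BP is a grabbable goggles prop that a hand can pick up and drop, with a toggleable highlight outline.
; OnGrab turns off mesh physics, attaches to the passed-in hand keeping world transform, and sets IsCatch.
; OnDrop restores physics, detaches the mesh and clears IsCatch.
; OpenOutline and CloseOutline toggle the mesh's custom depth rendering, which starts off at BeginPlay.
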(event `self.ReceiveBeginPlay`
  (set `self.IsCatch?` false)
  (`PrimitiveComponent.SetRenderCustomDepth` (`self.StaticMesh`) false))

(event `/Game/Player/moni/shiqulei/GrabBable.OnGrab`
  (params (Hand :type "SceneComponent Object Reference"))
  (`PrimitiveComponent.SetSimulatePhysics` (`self.StaticMesh`) false)
  (`self.K2_AttachToComponent` Hand "None" "KeepWorld" "KeepWorld" "KeepWorld")
  (set `self.IsCatch?` true))

(event `/Game/Player/moni/shiqulei/GrabBable.OnDrop`
  (`PrimitiveComponent.SetSimulatePhysics` (`self.StaticMesh`) true)
  (`SceneComponent.K2_DetachFromComponent` (`self.StaticMesh`) "KeepWorld" "KeepWorld" "KeepWorld" true)
  (set `self.IsCatch?` false))

(event `OpenOutline`
  (`PrimitiveComponent.SetRenderCustomDepth` (`self.StaticMesh`) true))

(event `CloseOutline`
  (if (`PrimitiveComponent.bRenderCustomDepth` (`self.StaticMesh`))
    (`PrimitiveComponent.SetRenderCustomDepth` (`self.StaticMesh`) false)))

(fn `UserConstructionScript`)
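; Collection point for a VR simulation that tracks pickup of five kit items: goggles, sprayer tank, sprayer hose, thermometer gun and first-aid kit.
; Sphere overlap casts the actor to each item class, sets that item's flag and increments the 完成量 counter once per type.
; Tick polls the counter and, at five, fires the "ce 收集完成" (collection complete) console event once.
; BeginPlay caches the SimVR_BP player, which is otherwise unused here.
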(event `self.ReceiveBeginPlay`
  (bind _assim_vr_bp (cast `/Game/Player/moni/PCcontrol/SimVR_BP` (`GameplayStatics.GetPlayerCharacter` 0)))
  (set `self.Player` _assim_vr_bp))

(event `self.ReceiveTick`
  (params (DeltaSeconds :type "Float (single-precision)"))
  (if (== (`self.完成量`) 5)
    (`/Engine/EditorBlueprintResources/StandardMacros.DoOnce` false
      (:`Completed`
        (`KismetSystemLibrary.ExecuteConsoleCommand` " ce 收集完成" null)))))

(event `self.Sphere.OnComponentBeginOverlap`
  (params (OverlappedComponent :type "PrimitiveComponent Object Reference") (OtherActor :type "Actor Object Reference") (OtherComp :type "PrimitiveComponent Object Reference") (OtherBodyIndex :type Integer) (bFromSweep :type Boolean) (SweepResult :type "HitResult Structure (by ref)"))
  (`|ExecutionSequence`
    (:`then_0`
      (bind _ashumujing_bp (cast `/Game/Player/moni/shiqulei/humujing_BP` OtherActor))
      (`KismetSystemLibrary.PrintString` "护目镜")
      (set `/Game/Player/moni/shiqulei/humujing_BP.护目镜` true _ashumujing_bp)
      (`/Engine/EditorBlueprintResources/StandardMacros.DoOnce` false
        (:`Completed`
          (set `self.完成量` (+ (`self.完成量`) 1)))))
    (:`then_1`
      (bind _aspenwuqi_shouji_bp (cast `/Game/Player/moni/shiqulei/penwuqi_shouji_BP` OtherActor))
      (`KismetSystemLibrary.PrintString` "喷雾箱")
      (set `/Game/Player/moni/shiqulei/penwuqi_shouji_BP.喷雾箱` true _aspenwuqi_shouji_bp)
      (`/Engine/EditorBlueprintResources/StandardMacros.DoOnce` false
        (:`Completed`
          (set `self.完成量` (+ (`self.完成量`) 1)))))
    (:`then_2`
      (bind _aspenwuqiguanzi_bp (cast `/Game/Player/moni/shiqulei/penwuqiguanzi_BP` OtherActor))
      (`KismetSystemLibrary.PrintString` "喷雾器管子")
      (set `/Game/Player/moni/shiqulei/penwuqiguanzi_BP.喷雾器管子` true _aspenwuqiguanzi_bp)
      (`/Engine/EditorBlueprintResources/StandardMacros.DoOnce` false
        (:`Completed`
          (set `self.完成量` (+ (`self.完成量`) 1)))))
    (:`then_3`
      (bind _ascewenqiangcollect_bp (cast `/Game/Player/moni/shiqulei/cewenqiangcollect_BP` OtherActor))
      (`KismetSystemLibrary.PrintString` "测温枪")
      (set `/Game/Player/moni/shiqulei/cewenqiangcollect_BP.测温枪` true _ascewenqiangcollect_bp)
      (`/Engine/EditorBlueprintResources/StandardMacros.DoOnce` false
        (:`Completed`
          (set `self.完成量` (+ (`self.完成量`) 1)))))
    (:`then_4`
      (bind _asjijiubao_bp (cast `/Game/Player/moni/shiqulei/jijiubao_BP` OtherActor))
      (`KismetSystemLibrary.PrintString` "急救包")
      (set `/Game/Player/moni/shiqulei/jijiubao_BP.急救包` true _asjijiubao_bp)
      (`/Engine/EditorBlueprintResources/StandardMacros.DoOnce` false
        (:`Completed`
          (set `self.完成量` (+ (`self.完成量`) 1)))))))

(fn `UserConstructionScript`)
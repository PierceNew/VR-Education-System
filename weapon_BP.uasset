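; Weapon Blueprint that builds on a grabbable parent class and realigns its mesh when a hand grabs it.
; On grab it calls the parent logic, then sets the StaticMesh relative location and rotation to the negated values of the Arrow component's relative transform.
; The Arrow thus serves as a grip marker, with component-wise negation used instead of a full transform inverse.
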(event `self.OnGrab`
  (params (Hand :type "SceneComponent Object Reference"))
  (bind _staticmesh (`self.StaticMesh`))
  (bind _arrow (`self.Arrow`))
  (`parent.OnGrab` Hand)
  (`SceneComponent.K2_SetRelativeLocation` _staticmesh (* (`SceneComponent.RelativeLocation` _arrow) -1.0) false false)
  (`SceneComponent.K2_SetRelativeRotation` _staticmesh (`KismetMathLibrary.NegateRotator` (`SceneComponent.RelativeRotation` _arrow)) false false))

(fn `UserConstructionScript`
  (`parent.UserConstructionScript`))